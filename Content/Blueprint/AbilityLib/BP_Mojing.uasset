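; BP_Mojing is a card ability that lets its card act as a wildcard for triples of other cards with Star 4 or higher.
; When obtained, it registers in the game's per-ID card dictionary and, unless it completes its own triple, joins eligible groups.
; When a qualifying minion is obtained later, the card joins that group too.
; Any group reaching three sets the triple flag, moves to the triple list and clears.
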(event `/Game/Blueprint/Interface/IN_Ability.获得此牌时`
  (params (card :type "/Game/Blueprint/Old/BP_Card Object Reference"))
  (bind _gameref (`self.gameref`))
  (bind _gameref_2 (`self.gameref`))
  (bind _id (`/Game/Blueprint/Old/BP_Card.id` card))
  (bind _carddic (`/Game/Blueprint/Old/BP_Game.carddic` (`self.gameref`)))
  (bind _cards (`/Game/Blueprint/Cards.cards` (`BlueprintMapLibrary.Map_Find` _carddic _id)))
  (if (not (`BlueprintMapLibrary.Map_Contains` _carddic _id))
    (bind _returnvalue (`|GenericCreateObject` "/Game/Blueprint/Cards.Cards_C"))
    (`BlueprintMapLibrary.Map_Add` _carddic _id _returnvalue))
  (`KismetArrayLibrary.Array_Add` _cards card)
  (if (== (`KismetArrayLibrary.Array_Length` _cards) 3)
    (set `/Game/Blueprint/Old/BP_Game.hastriple` true _gameref)
    (`KismetArrayLibrary.Array_Append` (`/Game/Blueprint/Old/BP_Game.triplelist` (`self.gameref`)) _cards)
    (`KismetArrayLibrary.Array_Clear` _cards)
    (else
      (bind _values (`BlueprintMapLibrary.Map_Values` (`/Game/Blueprint/Old/BP_Game.carddic` _gameref)))
      (for _array_element _values
        (bind _cards_2 (`/Game/Blueprint/Cards.cards` _array_element))
        (bind _output (`|GetArrayItem` _cards_2))
        (if (and (`KismetStringLibrary.NotEqual_StrStr` (`/Game/Blueprint/Old/BP_Card.id` (`self.cardref`)) (`/Game/Blueprint/Old/BP_Card.id` _output)) (>= (`/Game/Blueprint/Old/BP_Card.star` _output) 4))
          (`KismetArrayLibrary.Array_Add` _cards_2 card)
          (if (== (`KismetArrayLibrary.Array_Length` _cards_2) 3)
            (set `/Game/Blueprint/Old/BP_Game.hastriple` true _gameref_2)
            (`KismetArrayLibrary.Array_Append` (`/Game/Blueprint/Old/BP_Game.triplelist` _gameref_2) _cards_2)
            (`KismetArrayLibrary.Array_Clear` _cards_2)
            (`KismetArrayLibrary.Array_Clear` _cards)
            (break)))))))

(event `/Game/Blueprint/Interface/IN_Ability.获得随从牌时`
  (params (card :type "/Game/Blueprint/Old/BP_Card Object Reference"))
  (bind _gameref (`self.gameref`))
  (bind _id (`/Game/Blueprint/Old/BP_Card.id` card))
  (bind _cards (`/Game/Blueprint/Cards.cards` (`BlueprintMapLibrary.Map_Find` (`/Game/Blueprint/Old/BP_Game.carddic` (`self.gameref`)) _id)))
  (if (and (>= (`/Game/Blueprint/Old/BP_Card.star` card) 4) (`KismetStringLibrary.NotEqual_StrStr` _id (`/Game/Blueprint/Old/BP_Card.id` (`self.cardref`))))
    (`KismetArrayLibrary.Array_Add` _cards (`self.cardref`))
    (if (== (`KismetArrayLibrary.Array_Length` _cards) 3)
      (set `/Game/Blueprint/Old/BP_Game.hastriple` true _gameref)
      (`KismetArrayLibrary.Array_Append` (`/Game/Blueprint/Old/BP_Game.triplelist` _gameref) _cards)
      (`KismetArrayLibrary.Array_Clear` _cards)
      (`KismetArrayLibrary.Array_Clear` (`/Game/Blueprint/Cards.cards` (`BlueprintMapLibrary.Map_Find` (`/Game/Blueprint/Old/BP_Game.carddic` (`self.gameref`)) (`/Game/Blueprint/Old/BP_Card.id` (`self.cardref`))))))))