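; FL_Common is a function library of shared UI helpers for filling in widgets.
; SetText writes an integer as text, and SetIcon applies a texture to an image brush without matching its size.
; SetStar takes a 1-based index into a sprite array and builds the widget brush from that sprite.
; GetGameRef only returns false.
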(fn `GetGameRef`
  (returns (NewParam :type Boolean))
  (return false))

(fn `SetIcon`
  (params (widget :type "Image Object Reference") (texture :type "Texture2D Object Reference"))
  (`Image.SetBrushFromTexture` widget texture false))

(fn `SetStar`
  (params (widget :type "Image Object Reference") (spritearray :type "Array of PaperSprite Object Reference") (index :type Integer))
  (`Image.SetBrush` widget (`PaperSpriteBlueprintLibrary.MakeBrushFromSprite` (`|GetArrayItem` spritearray (- index 1)))))

(fn `SetText`
  (params (widget :type "TextBlock Object Reference") (info :type Integer))
  (`TextBlock.SetText` widget (`KismetTextLibrary.Conv_IntToText` info)))