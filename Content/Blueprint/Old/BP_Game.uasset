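; Game manager for a card auto-battler prototype, handling the shop, hand, board, tavern-style leveling and merging of triples into gold cards.
; Battles spawn three random enemies and copies of field cards, then alternate timeline-lerped attacks on random targets, front slots first.
; Each battle outcome starts a new turn, with losses costing hero health.
; UI updates, initial shop refresh and timer expiry are disconnected, and panel switching is empty.
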(event `self.ReceiveBeginPlay`
  (`WidgetComponent.SetDrawSize` (`self.Widget`) (1080.0 2340.0)))

(event `三连`
  (bind _handlist (`self.handlist`))
  (bind _triplelist (`self.triplelist`))
  (`KismetSystemLibrary.PrintString` "三连了！！！")
  (bind _returnvalue (`|SpawnActorFromClass` "/Game/Blueprint/Old/BP_Card.BP_Card_C" (`KismetMathLibrary.MakeTransform` (0.0 0.0 0.0)) "AlwaysSpawn" "OverrideRootScale" null null))
  (`/Game/Blueprint/Old/BP_Card.初始化卡牌` _returnvalue self (`KismetStringLibrary.Conv_StringToName` (`/Game/Blueprint/Old/BP_Card.id` (`|GetArrayItem` (`self.triplelist`)))) true)
  (`self.合并属性` _triplelist _returnvalue)
  (for _array_element _triplelist
    (if (`KismetArrayLibrary.Array_Contains` _handlist _array_element)
      (`KismetArrayLibrary.Array_RemoveItem` _handlist _array_element))
    (`self.K2_DestroyActor` _array_element))
  (`KismetArrayLibrary.Array_Clear` _triplelist)
  (`BlueprintMapLibrary.Map_Remove` (`self.carddic`) (`/Game/Blueprint/Old/BP_Card.id` _returnvalue))
  (bind _returnvalue_2 (`KismetArrayLibrary.Array_Add` (`self.handlist`) _returnvalue))
  (set `/Game/Blueprint/Old/BP_Card.isinhand` true _returnvalue)
  (bind _output (`|GetArrayItem` (`self.handslots`) _returnvalue_2))
  (`self.K2_SetActorLocation` _returnvalue _output false false)
  (set `/Game/Blueprint/Old/BP_Card.cardlocation` _output _returnvalue))

(event `开始计时`
  (bind _returnvalue (`KismetSystemLibrary.K2_SetTimerDelegate` (delegate `计时`) 1.0 true)))

(event `计时`
  (bind _output_get (set `self.turntimes` (- (`self.turntimes`) 1))))

(event `升级`
  (if (and (< (`self.level`) 6) (>= (`self.curcoins`) (`self.levelupcost`)))
    (set `self.curcoins` (- (`self.curcoins`) (`self.levelupcost`)))
    (set `self.level` (+ (`self.level`) 1))
    (set `self.levelupcost` (+ (`self.level`) 5))))

(event `刷新`
  (bind _shoplist (`self.shoplist`))
  (if (> (`KismetArrayLibrary.Array_Length` (`self.shoplist`)) 0)
    (for _array_element _shoplist
      (`self.K2_DestroyActor` _array_element))
    (`KismetArrayLibrary.Array_Clear` _shoplist))
  (for _index (range 3)
    (bind _returnvalue (`DataTableFunctionLibrary.GetDataTableColumnAsString` "/Game/Data/DT_Card.DT_Card" "id"))
    (bind _output (`|GetArrayItem` (`self.shopslots`) _index))
    (bind _returnvalue_2 (`|SpawnActorFromClass` "/Game/Blueprint/Old/BP_Card.BP_Card_C" (`KismetMathLibrary.MakeTransform` _output) "AlwaysSpawn" "OverrideRootScale" null null))
    (`/Game/Blueprint/Old/BP_Card.初始化卡牌` _returnvalue_2 self (`KismetStringLibrary.Conv_StringToName` (`KismetArrayLibrary.Array_Random` _returnvalue)) false)
    (set `/Game/Blueprint/Old/BP_Card.cardlocation` _output _returnvalue_2)
    (`KismetArrayLibrary.Array_Add` (`self.shoplist`) _returnvalue_2)))

(event `锁定`
  (bind _shoplist (`self.shoplist`))
  (if (`self.islock`)
    (for _array_element _shoplist
      _)
    (set `self.islock` false)
    (else
      (for _array_element_2 _shoplist
        _)
      (set `self.islock` true))))

(event `购买卡牌`
  (params (card :type "/Game/Blueprint/Old/BP_Card Object Reference (by ref)"))
  (`KismetArrayLibrary.Array_RemoveItem` (`self.shoplist`) card)
  (message `/Game/Blueprint/Interface/IN_Card.购买时` card null)
  (if (`self.hastriple`)
    (`self.三连`)
    (set `self.hastriple` false)
    (else
      (bind _returnvalue (`KismetArrayLibrary.Array_Add` (`self.handlist`) card))
      (set `/Game/Blueprint/Old/BP_Card.isinhand` true card)
      (bind _output (`|GetArrayItem` (`self.handslots`) _returnvalue))
      (`self.K2_SetActorLocation` card _output false false)
      (set `/Game/Blueprint/Old/BP_Card.cardlocation` _output card))))

(event `出售卡牌`
  (params (card :type "/Game/Blueprint/Old/BP_Card Object Reference"))
  (if (`/Game/Blueprint/Old/BP_Card.isinhand` card)
    (`KismetArrayLibrary.Array_RemoveItem` (`self.handlist`) card))
  (message `/Game/Blueprint/Interface/IN_Card.出售时` card null)
  (`self.K2_DestroyActor` card))

(event `使用卡牌`
  (params (card :type "/Game/Blueprint/Old/BP_Card Object Reference") (index :type Integer))
  (bind _fieldlist (`self.fieldlist`))
  (bind _output (`|GetArrayItem` _fieldlist index))
  (`/Engine/EditorBlueprintResources/StandardMacros.IsValid` _output
    (:`Is Valid`
      (for (_array_element _array_index) _fieldlist
        (`/Engine/EditorBlueprintResources/StandardMacros.IsValid` _array_element
          (:`Is Not Valid`
            (`KismetArrayLibrary.Array_Set` (`self.fieldlist`) _array_index _output)
            (`self.K2_SetActorLocation` _output (`|GetArrayItem` (`self.fieldslots`) _array_index) false false)
            (break)))))
    (:`Is Not Valid`
      _))
  (`KismetArrayLibrary.Array_Set` (`self.fieldlist`) index card)
  (`KismetArrayLibrary.Array_RemoveItem` (`self.handlist`) card)
  (message `/Game/Blueprint/Interface/IN_Card.使用时` card null))

(event `交换位置`
  (params (card :type "/Game/Blueprint/Old/BP_Card Object Reference") (index :type Integer))
  (bind _fieldlist (`self.fieldlist`))
  (bind _returnvalue (`KismetArrayLibrary.Array_Find` _fieldlist card))
  (bind _output (`|GetArrayItem` _fieldlist index))
  (`/Engine/EditorBlueprintResources/StandardMacros.IsValid` _output
    (:`Is Valid`
      (`self.K2_SetActorLocation` _output (`|GetArrayItem` (`self.fieldslots`) _returnvalue) false false)
      (`KismetArrayLibrary.Array_Swap` _fieldlist index _returnvalue))))

(event `回合结束`
  (`KismetSystemLibrary.Delay` 0.5)
  (bind _output_get (set `self.isbattle` true))
  (`self.切换面板` _output_get)
  (`self.战斗开始`)
  (`KismetSystemLibrary.Delay` 0.5)
  (`self.开始战斗`))

(event `回合开始`
  (`KismetSystemLibrary.Delay` 0.5)
  (bind _output_get (set `self.isbattle` false))
  (`self.切换面板` _output_get)
  (set `self.turntimes` 10)
  (`self.开始计时`)
  (if (`self.islock`)
    (`self.锁定`)
    (else
      (`self.刷新`))))

(event `战斗开始`
  (for _index (range 3)
    (bind _returnvalue (`DataTableFunctionLibrary.GetDataTableColumnAsString` "/Game/Data/DT_Card.DT_Card" "id"))
    (bind _output (`|GetArrayItem` (`self.enemyslots`) _index))
    (bind _returnvalue_2 (`|SpawnActorFromClass` "/Game/Blueprint/Old/BP_Card.BP_Card_C" (`KismetMathLibrary.MakeTransform` _output) "AlwaysSpawn" "OverrideRootScale" null null))
    (`/Game/Blueprint/Old/BP_Card.随机生成随从` _returnvalue_2 self (`KismetStringLibrary.Conv_StringToName` (`KismetArrayLibrary.Array_Random` _returnvalue)))
    (set `/Game/Blueprint/Old/BP_Card.cardlocation` _output _returnvalue_2)
    (`KismetArrayLibrary.Array_Set` (`self.enemylist`) _index _returnvalue_2))
  (for (_array_element _array_index) (`self.fieldlist`)
    (`/Engine/EditorBlueprintResources/StandardMacros.IsValid` _array_element
      (:`Is Valid`
        (bind _output_2 (`|GetArrayItem` (`self.friendlyslots`) _array_index))
        (bind _returnvalue_3 (`|SpawnActorFromClass` "/Game/Blueprint/Old/BP_Card.BP_Card_C" (`KismetMathLibrary.MakeTransform` _output_2) "AlwaysSpawn" "OverrideRootScale" null null))
        (`/Game/Blueprint/Old/BP_Card.同步生成随从` _returnvalue_3 self (`/Game/Blueprint/Old/BP_Card.star` _array_element) null (`/Game/Blueprint/Old/BP_Card.attack` _array_element) (`/Game/Blueprint/Old/BP_Card.health` _array_element))
        (set `/Game/Blueprint/Old/BP_Card.cardlocation` _output_2 _returnvalue_3)
        (`KismetArrayLibrary.Array_Set` (`self.friendlylist`) _array_index _returnvalue_3)))))

(event `开始战斗`
  (bind _output (`|GetArrayItem` (`self.enemylist`) (`self.curenemy`)))
  (bind _output_2 (`|GetArrayItem` (`self.friendlylist`) (`self.curfriendly`)))
  (bind _output_3 (`|GetArrayItem` (`self.enemylist`) (`self.curenemy`)))
  (bind _output_4 (`|GetArrayItem` (`self.enemylist`) (`self.target`)))
  (bind _output_5 (`|GetArrayItem` (`self.friendlylist`) (`self.target`)))
  (bind _output_6 (`|GetArrayItem` (`self.friendlylist`) (`self.curfriendly`)))
  (`self.判断战斗结算`
    (:`继续战斗`
      (if (`KismetMathLibrary.RandomBool`)
        (`/Engine/EditorBlueprintResources/StandardMacros.IsValid` _output_6 :!label _label
          (:`Is Valid`
            (bind _target (`self.选择攻击目标` (`self.enemylist`)))
            (set `self.target` _target)
            (bind (_direction _value) (`Timeline|攻击轨迹插值` :!via `PlayFromStart`)
              (:`Update`
                (`self.K2_SetActorLocation` _output_6 (`KismetMathLibrary.VLerp` (`|GetArrayItem` (`self.friendlyslots`) (`self.curfriendly`)) (`|GetArrayItem` (`self.enemyslots`) (`self.target`)) _value) false false))
              (:`Finished`
                (bind _isdead (`/Game/Blueprint/Old/BP_Card.结算伤害` _output_4 (`|GetArrayItem` (`self.friendlylist`) (`self.curfriendly`))))
                (bind _isdead_2 (`/Game/Blueprint/Old/BP_Card.结算伤害` _output_2 (`|GetArrayItem` (`self.enemylist`) (`self.target`))))
                (`/Game/Blueprint/Old/BP_Card.结算死亡` _output_2 _isdead_2)
                (`/Game/Blueprint/Old/BP_Card.结算死亡` _output_4 _isdead)
                (`self.判断战斗结算`
                  (:`继续战斗`
                    (`self.设置当前友方`)
                    (`/Engine/EditorBlueprintResources/StandardMacros.IsValid` _output :!label _label_2
                      (:`Is Valid`
                        (bind _target_2 (`self.选择攻击目标` (`self.friendlylist`)))
                        (set `self.target` _target_2)
                        (bind (_direction_2 _value_2) (`Timeline|时间轴` :!via `PlayFromStart`)
                          (:`Update`
                            (`self.K2_SetActorLocation` _output (`KismetMathLibrary.VLerp` (`|GetArrayItem` (`self.enemyslots`) (`self.curenemy`)) (`|GetArrayItem` (`self.friendlyslots`) (`self.target`)) _value_2) false false))
                          (:`Finished`
                            (bind _isdead_3 (`/Game/Blueprint/Old/BP_Card.结算伤害` _output_5 (`|GetArrayItem` (`self.enemylist`) (`self.curenemy`))))
                            (bind _isdead_4 (`/Game/Blueprint/Old/BP_Card.结算伤害` _output_3 (`|GetArrayItem` (`self.friendlylist`) (`self.target`))))
                            (`/Game/Blueprint/Old/BP_Card.结算死亡` _output_3 _isdead_4)
                            (`/Game/Blueprint/Old/BP_Card.结算死亡` _output_5 _isdead_3)
                            (`self.判断战斗结算`
                              (:`继续战斗`
                                (`self.设置当前敌方`)
                                (goto _label))
                              (:`敌方胜利`
                                (`self.结算英雄伤害` null)
                                (`self.清空场地` (`self.enemylist`)))
                              (:`我方胜利`
                                (`self.清空场地` (`self.friendlylist`)))
                              (:`平局`
                                _))
                            (`self.回合开始`))))
                      (:`Is Not Valid`
                        (`self.设置当前敌方`)
                        (goto _label_2))))
                  (:`敌方胜利`
                    (`self.结算英雄伤害` null)
                    (`self.清空场地` (`self.enemylist`))
                    (`self.回合开始` :!label _label_3))
                  (:`我方胜利`
                    (`self.清空场地` (`self.friendlylist`))
                    (goto _label_3))
                  (:`平局`
                    (goto _label_3))))))
          (:`Is Not Valid`
            (`self.设置当前友方`)
            (goto _label)))
        (else
          (goto _label_2))))
    (:`敌方胜利`
      (`self.结算英雄伤害` null)
      (`self.清空场地` (`self.enemylist`))
      (`self.回合开始` :!label _label_4))
    (:`我方胜利`
      (`self.清空场地` (`self.friendlylist`))
      (goto _label_4))
    (:`平局`
      (goto _label_4))))

(fn `UserConstructionScript`)

(fn `切换面板`
  (params (isbattle :type Boolean)))

(fn `合并属性`
  (params (cards :type "Array of /Game/Blueprint/Old/BP_Card Object Reference") (target :type "/Game/Blueprint/Old/BP_Card Object Reference"))
  (locals (attack :type Integer) (health :type Integer))
  (for _array_element cards
    (set `local.attack` (- (+ (`/Game/Blueprint/Old/BP_Card.attack` _array_element) (`local.attack`)) (`/Game/Blueprint/Old/BP_Card.attackbase` _array_element)))
    (set `local.health` (- (+ (`/Game/Blueprint/Old/BP_Card.health` _array_element) (`local.health`)) (`/Game/Blueprint/Old/BP_Card.healthbase` _array_element))))
  (set `/Game/Blueprint/Old/BP_Card.attack` (+ (`local.attack`) (* (`/Game/Blueprint/Old/BP_Card.attack` target) 2)) target)
  (set `/Game/Blueprint/Old/BP_Card.health` (+ (`local.health`) (* (`/Game/Blueprint/Old/BP_Card.health` target) 2)) target))

(fn `添加卡牌`
  (params (card :type "/Game/Blueprint/Old/BP_Card Object Reference"))
  (locals (value :type "/Game/Blueprint/Structure/ST_CardList Structure"))
  (bind _carddic (`self.carddic`))
  (bind _id (`/Game/Blueprint/Old/BP_Card.id` card))
  (bind _cards (`/Game/Blueprint/Cards.cards` (`BlueprintMapLibrary.Map_Find` _carddic _id)))
  (if (not (`BlueprintMapLibrary.Map_Contains` _carddic _id))
    (bind _returnvalue (`|GenericCreateObject` "/Game/Blueprint/Cards.Cards_C"))
    (`BlueprintMapLibrary.Map_Add` _carddic _id _returnvalue))
  (`KismetArrayLibrary.Array_Add` _cards card)
  (if (== (`KismetArrayLibrary.Array_Length` _cards) (`self.triplecount`))
    _))

(fn `清空场地`
  (params (list :type "Array of /Game/Blueprint/Old/BP_Card Object Reference"))
  (for _array_element list
    (`/Engine/EditorBlueprintResources/StandardMacros.IsValid` _array_element
      (:`Is Valid`
        (`self.K2_DestroyActor` _array_element)))))

(fn `移除卡牌`
  (params (card :type "/Game/Blueprint/Old/BP_Card Object Reference"))
  (locals (value :type "/Game/Blueprint/Structure/ST_CardList Structure"))
  (`KismetArrayLibrary.Array_RemoveItem` (`/Game/Blueprint/Cards.cards` (`BlueprintMapLibrary.Map_Find` (`self.carddic`) (`/Game/Blueprint/Old/BP_Card.id` card))) card))

(fn `结算英雄伤害`
  (params (player :type "/Game/Blueprint/Old/BP_Game Object Reference"))
  (returns (isdead :type Boolean))
  (locals (damage :type Integer))
  (for _array_element (`self.enemylist`)
    (`/Engine/EditorBlueprintResources/StandardMacros.IsValid` _array_element
      (:`Is Valid`
        (set `local.damage` (+ (`local.damage`) (`/Game/Blueprint/Old/BP_Card.star` _array_element))))))
  (bind _output_get (set `local.damage` (+ (`local.damage`) (`self.level`))))
  (bind _output_get_2 (set `self.health` (- (`self.health`) _output_get))))

(fn `设置当前友方`
  (bind _curfriendly (`self.curfriendly`))
  (set `self.curfriendly` (+ _curfriendly 1))
  (if (== _curfriendly 6)
    (set `self.curfriendly` 0)))

(fn `设置当前敌方`
  (bind _curenemy (`self.curenemy`))
  (set `self.curenemy` (+ _curenemy 1))
  (if (== _curenemy 6)
    (set `self.curenemy` 0)))

(fn `选择攻击目标`
  (params (list :type "Array of /Game/Blueprint/Old/BP_Card Object Reference"))
  (returns (target :type Integer))
  (locals (validtarget :type "Array of Integer"))
  (bind _validtarget (`local.validtarget`))
  (bind _outitem (`KismetArrayLibrary.Array_Random` _validtarget))
  (for _index (range 3)
    (`/Engine/EditorBlueprintResources/StandardMacros.IsValid` (`|GetArrayItem` list _index)
      (:`Is Valid`
        (`KismetArrayLibrary.Array_Add` (`local.validtarget`) _index))))
  (if (`KismetArrayLibrary.Array_IsNotEmpty` _validtarget)
    (return _outitem)
    (else
      (for _index_2 (range 3 6)
        (`/Engine/EditorBlueprintResources/StandardMacros.IsValid` (`|GetArrayItem` list _index_2)
          (:`Is Valid`
            (`KismetArrayLibrary.Array_Add` (`local.validtarget`) _index_2))))
      (return _outitem))))