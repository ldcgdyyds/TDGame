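; BP_Card is a card/minion actor for a card game with a shop, hand and field, using a widget component as its face.
; Init events read Star from DT_Card or parameters; minion variants swap in a WB_Creature widget.
; Play, buy and sell events call Ability hooks, with purchases also notifying field and hand cards.
; Damage and death functions exist, but stat assignment, Ability construction and the death check are disconnected.
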(event `初始化卡牌`
  (params (game :type "/Game/Blueprint/Old/BP_Game Object Reference") (RowName :type Name) (gold :type Boolean))
  (bind _output_get (set `self.gameref` game))
  (bind _aswb_card (cast `/Game/UI/Old/WB_Card` (`WidgetComponent.GetWidget` (`self.Widget`))))
  (set `self.UIcard` _aswb_card)
  (bind _returnvalue (`|GetDataTableRow` "/Game/Data/DT_Card.DT_Card" RowName)
    (:`then`
      (bind (_id _name _logic _star _icon _attack _health) (break `/Game/Blueprint/Structure/ST_Card` _returnvalue))
      (set `self.id` _id)
      (set `self.star` _star))))

(event `同步卡牌`
  (params (game :type "/Game/Blueprint/Old/BP_Game Object Reference") (star :type Integer) (icon :type "PaperSprite Object Reference") (attack :type Integer) (health :type Integer))
  (set `self.gameref` game)
  (set `self.star` star))

(event `随机生成随从`
  (params (game :type "/Game/Blueprint/Old/BP_Game Object Reference") (RowName :type Name))
  (set `self.gameref` game)
  (`self.初始化随从`)
  (bind _returnvalue (`|GetDataTableRow` "/Game/Data/DT_Card.DT_Card" RowName)
    (:`then`
      (set `self.star` (`.star_19_8D49D57341B507C9DE3F5185C5D0EA29` (break `/Game/Blueprint/Structure/ST_Card` _returnvalue))))))

(event `同步生成随从`
  (params (game :type "/Game/Blueprint/Old/BP_Game Object Reference") (star :type Integer) (icon :type "PaperSprite Object Reference") (attack :type Integer) (health :type Integer))
  (`self.初始化随从`)
  (set `self.gameref` game)
  (set `self.star` star))

(event `转化生成随从`
  (`self.初始化随从`))

(event `/Game/Blueprint/Interface/IN_Card.使用时`
  (params (card :type "/Game/Blueprint/Old/BP_Card Object Reference"))
  (`/Game/Blueprint/Old/BP_Ability.入场` (`self.ability`) self))

(event `/Game/Blueprint/Interface/IN_Card.购买时`
  (params (card :type "/Game/Blueprint/Old/BP_Card Object Reference"))
  (bind _gameref (`self.gameref`))
  (message `/Game/Blueprint/Interface/IN_Ability.获得此牌时` (`self.ability`) self)
  (for _array_element (`/Game/Blueprint/Old/BP_Game.fieldlist` _gameref)
    (`/Engine/EditorBlueprintResources/StandardMacros.IsValid` _array_element
      (:`Is Valid`
        (message `/Game/Blueprint/Interface/IN_Ability.获得随从牌时` (`/Game/Blueprint/Old/BP_Card.ability` _array_element) self))))
  (for _array_element_2 (`/Game/Blueprint/Old/BP_Game.handlist` _gameref)
    (message `/Game/Blueprint/Interface/IN_Ability.获得随从牌时` (`/Game/Blueprint/Old/BP_Card.ability` _array_element_2) self)))

(event `/Game/Blueprint/Interface/IN_Card.出售时`
  (params (card :type "/Game/Blueprint/Old/BP_Card Object Reference"))
  (message `/Game/Blueprint/Interface/IN_Ability.失去此牌时` (`self.ability`) self))

(fn `UserConstructionScript`)

(fn `初始化随从`
  (returns (UI :type "/Game/UI/Old/WB_Creature Object Reference"))
  (bind _widget (`self.Widget`))
  (bind _returnvalue (`|CreateWidget` "/Game/UI/Old/WB_Creature.WB_Creature_C"))
  (`WidgetComponent.SetWidget` _widget _returnvalue)
  (`WidgetComponent.SetDrawSize` _widget (210.0 280.0))
  (bind _output_get (set `self.UIcreature` _returnvalue))
  (return _output_get))

(fn `结算伤害`
  (params (card :type "/Game/Blueprint/Old/BP_Card Object Reference"))
  (returns (isdead :type Boolean))
  (bind _output_get (set `self.health` (- (`self.health`) (`/Game/Blueprint/Old/BP_Card.attack` card)))))

(fn `结算死亡`
  (params (isdead :type Boolean))
  (if isdead
    (`self.K2_DestroyActor`)))