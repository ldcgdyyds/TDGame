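; BP_Ability is a card ability object that tracks owned copies of cards and provides an on-entry (入场) buff.
; Initialization stores game and card references; gain and lose events add or remove cards in the game's Id-keyed dictionary.
; A third matching copy sets the game's triple flag, moves that group to the triple list and clears it.
; The 入场 function gives the passed card +1 attack and +1 health.
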(event `初始化能力`
  (params (game :type "/Game/Blueprint/Old/BP_Game Object Reference") (card :type "/Game/Blueprint/Old/BP_Card Object Reference"))
  (set `self.gameref` game)
  (set `self.cardref` card))

(event `/Game/Blueprint/Interface/IN_Ability.获得此牌时`
  (params (card :type "/Game/Blueprint/Old/BP_Card Object Reference"))
  (bind _gameref (`self.gameref`))
  (bind _id (`/Game/Blueprint/Old/BP_Card.id` card))
  (bind _carddic (`/Game/Blueprint/Old/BP_Game.carddic` (`self.gameref`)))
  (bind _cards (`/Game/Blueprint/Cards.cards` (`BlueprintMapLibrary.Map_Find` _carddic _id)))
  (if (not (`BlueprintMapLibrary.Map_Contains` _carddic _id))
    (bind _returnvalue (`|GenericCreateObject` "/Game/Blueprint/Cards.Cards_C"))
    (`BlueprintMapLibrary.Map_Add` _carddic _id _returnvalue))
  (`KismetArrayLibrary.Array_Add` _cards card)
  (if (== (`KismetArrayLibrary.Array_Length` _cards) 3)
    (set `/Game/Blueprint/Old/BP_Game.hastriple` true _gameref)
    (`KismetArrayLibrary.Array_Append` (`/Game/Blueprint/Old/BP_Game.triplelist` _gameref) _cards)
    (`KismetArrayLibrary.Array_Clear` _cards)))

(event `/Game/Blueprint/Interface/IN_Ability.失去此牌时`
  (params (card :type "/Game/Blueprint/Old/BP_Card Object Reference"))
  (`KismetArrayLibrary.Array_RemoveItem` (`/Game/Blueprint/Cards.cards` (`BlueprintMapLibrary.Map_Find` (`/Game/Blueprint/Old/BP_Game.carddic` (`self.gameref`)) (`/Game/Blueprint/Old/BP_Card.id` card))) card))

(fn `入场`
  (params (card :type "/Game/Blueprint/Old/BP_Card Object Reference"))
  (set `/Game/Blueprint/Old/BP_Card.attack` (+ (`/Game/Blueprint/Old/BP_Card.attack` card) 1) card)
  (set `/Game/Blueprint/Old/BP_Card.health` (+ (`/Game/Blueprint/Old/BP_Card.health` card) 1) card))